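; Base actor whose mesh can fade out and back in, likely for objects that need to be hidden temporarily.
; The Construction Script caches the original materials and creates dynamic instances from FadeMaterialInstances.
; FadeOut swaps these in and plays a timeline driving their Fade parameter, while FadeIn reverses it.
; Fully faded meshes ignore the Visibility channel; fully restored ones block it again and regain their original materials.
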(event `Fade Out`
  ;[1 1 1] fasdes out by adjusting the paremeter on the material to zero
  (`self.SetMaterialsToDynamicInstance`)
  (bind (_direction _fade) (`Timeline|FadeTimeline` :!label _label)
    (:`Update`
      (for _array_element (`self.DynamicMaterialInstance`)
        (`MaterialInstanceDynamic.SetScalarParameterValue` _array_element "Fade" _fade)))
    (:`Finished`
      ;[1 1 1] Resets the materials back to normal no fade material
      (if (>= _fade 1.0)
        (for (_array_element_2 _array_index) (`self.Original Materials`)
          (`PrimitiveComponent.SetMaterial` (`self.Mesh`) _array_index _array_element_2)
          ;[1 1 1] when fading block visibility
          (`PrimitiveComponent.SetCollisionResponseToChannel` (`self.Mesh`) "ECC_Visibility" "ECR_Block"))
        (else
          ;[1 1 1] when faded ignore visibility
          (if (<= _fade 0.0)
            (`PrimitiveComponent.SetCollisionResponseToChannel` (`self.Mesh`) "ECC_Visibility" "ECR_Ignore")))))))

(event `FadeIn`
  ;[1 1 1] fasdes out by adjusting the paremeter on the material to zero
  (goto _label :!via `Reverse`))

(event `self.ReceiveBeginPlay`)

(fn `SetMaterialsToDynamicInstance`
  (for (_array_element _array_index) (`self.DynamicMaterialInstance`)
    (`PrimitiveComponent.SetMaterial` (`self.Mesh`) _array_index _array_element)))

(fn `UserConstructionScript`
  (`KismetArrayLibrary.Array_Clear` (`self.DynamicMaterialInstance`))
  (set `self.Original Materials` (`MeshComponent.GetMaterials` (`self.Mesh`)))
  (for _array_element (`self.FadeMaterialInstances`)
    (bind _returnvalue (`KismetMaterialLibrary.CreateDynamicMaterialInstance` _array_element))
    (`KismetArrayLibrary.Array_AddUnique` (`self.DynamicMaterialInstance`) _returnvalue)))