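; Ranged enemy attack gameplay ability that fires a projectile at the avatar's combat target.
; On activation it caches the target's location, turns the avatar toward it through interface messages and plays a random tagged attack montage.
; A one-shot gameplay event matching the montage tag triggers SpawnProjectile toward the cached location.
; The graph never calls EndAbility, and an older last-montage variant remains unconnected.
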(event `self.K2_ActivateAbility`
  (bind _returnvalue (`self.GetAvatarActorFromActorInfo`))
  (bind _returnvalue_2 (message `MouseTargetInterface.GetCombatTarget` _returnvalue))
  (bind _output_get (set `self.TargetToAttackLocation` (`Actor.K2_GetActorLocation` _returnvalue_2)))
  (message `CombatInterface.UpdateFacingTarget` _returnvalue _output_get)
  (bind _returnvalue_3 (message `CombatInterface.GetAttackMontages` _returnvalue))
  (bind _output_get_2 (set `self.TaggedMontage` (`self.GetRandomTaggedMontageFromArray` _returnvalue_3)))
  (bind (_montage _montagetag) (break `TaggedMontage` _output_get_2))
  (`AbilityTask_PlayMontageAndWait.CreatePlayMontageAndWaitProxy` "None" _montage 1.0 "None" false
    (:`then`
      (`AbilityTask_WaitGameplayEvent.WaitGameplayEvent` _montagetag null true
        (:`EventReceived`
          (message `CombatInterface.GetCombatSocketLocation` (`self.GetAvatarActorFromActorInfo`) _montagetag)
          (`self.SpawnProjectile` (`self.TargetToAttackLocation`)))))))