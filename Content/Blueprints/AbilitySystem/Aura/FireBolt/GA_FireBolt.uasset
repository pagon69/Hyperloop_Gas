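; Fire Bolt gameplay ability that casts a projectile toward the target under the mouse.
; On activation it gets the cursor hit location, turns the avatar to face it through the C++ CombatInterface, and plays the cast montage.
; A montage gameplay event triggers the projectile spawn from the weapon socket, then the ability ends after a short delay.
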(event `self.K2_ActivateAbility`
  (bind (_asynctaskproxy _datahandle) (`TargetDataUnderMouse.CreateTargetDataUnderMouse`)
    (:`ValidData`
      (bind _output_get (set `self.ProjectileTargetLocation` (`.Location` (`GameplayStatics.BreakHitResult` (`AbilitySystemBlueprintLibrary.GetHitResultFromTargetData` _datahandle)))))
      ;[1 1 1] pulls from C++ interface
      (bind _ascombat_interface (cast `CombatInterface` (`self.GetAvatarActorFromActorInfo`)))
      (`CombatInterface.UpdateFacingTarget` _ascombat_interface _output_get)
      ;[1 1 1] plays montage and spawns firebolt
      (`AbilityTask_PlayMontageAndWait.CreatePlayMontageAndWaitProxy` "None" "/Game/Assets/Characters/Aura/Animations/Abilities/AM_Cast_Firebolt.AM_Cast_Firebolt"
        (:`then`
          (`AbilityTask_WaitGameplayEvent.WaitGameplayEvent` (struct :`TagName` "Event.Montage.FireBolt") null true
            (:`EventReceived`
              (`self.SpawnProjectile` (`self.ProjectileTargetLocation`) (`BlueprintGameplayTagLibrary.MakeLiteralGameplayTag` (struct :`TagName` "CombatSocket.Weapon")))
              (`KismetSystemLibrary.Delay` 0.5)
              (`self.K2_EndAbility`))))))))